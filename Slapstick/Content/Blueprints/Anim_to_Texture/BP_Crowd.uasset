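; Crowd actor that fills an instanced static mesh component with a grid of StaticMeshAsset copies.
; The construction script spaces instances by rows and columns, adding seeded random X jitter and yaw.
; AnimToTexture playback setup, which picks random DataAsset animations and writes per-instance custom data, is disconnected, leaving the final per-instance loop empty.
; The event graph has no active logic.
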(fn `UserConstructionScript`
  (bind _randomstream (`self.RandomStream`))
  (bind _maxangle (`self.MaxAngle`))
  ;[1 1 1] Comment
  (`|ExecutionSequence`
    (:`then_0`
      (`StaticMeshComponent.SetStaticMesh` (`self.InstancedStaticMesh`) (`self.StaticMeshAsset`)))
    (:`then_1`
      (for _index (range (`self.Rows`))
        (for _index_2 (range (`self.Columns`))
          (`InstancedStaticMeshComponent.AddInstance` (`self.InstancedStaticMesh`) (`KismetMathLibrary.MakeTransform` (`KismetMathLibrary.MakeVector` (+ (* _index_2 (`self.ColDistance`)) (`KismetMathLibrary.RandomFloatInRangeFromStream` _randomstream 0.0 (`self.ShuffleAmount`))) (* _index (`self.RowDistance`))) (`KismetMathLibrary.MakeRotator` 0.0 0.0 (`KismetMathLibrary.RandomFloatInRangeFromStream` _randomstream (* _maxangle -1.0) _maxangle))) false))))
    (:`then_2`
      (for _index_3 (range (* (`self.Rows`) (`self.Columns`)))
        _))))