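; BP_Hand is the slapping hand actor, which damages characters it touches.
; On Sphere1 overlap it prints the game instance's FVelocity, then subtracts that velocity times DamageMultiplier from the BP_ThirdPersonCharacter's Health.
; For each W_SlapMeter widget found, it pauses the meter animation, spawns BP_Force at the Sphere component and plays a slap sound.
; A ragdoll physics call on the character's mesh is left disconnected.
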(event `self.ReceiveTick`
  (params (DeltaSeconds :type "Float (single-precision)")))

(event `self.Sphere1.OnComponentBeginOverlap`
  (params (OverlappedComponent :type "PrimitiveComponent Object Reference") (OtherActor :type "Actor Object Reference") (OtherComp :type "PrimitiveComponent Object Reference") (OtherBodyIndex :type Integer) (bFromSweep :type Boolean) (SweepResult :type "HitResult Structure (by ref)"))
  (bind (_returnvalue_location _returnvalue_rotation) (`KismetMathLibrary.BreakTransform` (`SceneComponent.K2_GetComponentToWorld` (`self.Sphere`))))
  (`|ExecutionSequence`
    (:`then_0`
      (bind _asslapstick_game_inst (cast `/Game/Blueprints/SlapstickGameInst` (`GameplayStatics.GetGameInstance`)))
      (bind _fvelocity (`/Game/Blueprints/SlapstickGameInst.FVelocity` _asslapstick_game_inst))
      (`KismetSystemLibrary.PrintString` (`KismetStringLibrary.Conv_DoubleToString` _fvelocity)))
    (:`then_1`
      (bind _asbp_third_person_character (cast `/Game/ThirdPerson/Blueprints/BP_ThirdPersonCharacter` OtherActor))
      (set `/Game/ThirdPerson/Blueprints/BP_ThirdPersonCharacter.Health` (- (`/Game/ThirdPerson/Blueprints/BP_ThirdPersonCharacter.Health` _asbp_third_person_character) (* _fvelocity (`/Game/Blueprints/SlapstickGameInst.DamageMultiplier` (cast `/Game/Blueprints/SlapstickGameInst` (`GameplayStatics.GetGameInstance`) :!pure true)))) _asbp_third_person_character)
      (bind _foundwidgets (`WidgetBlueprintLibrary.GetAllWidgetsOfClass` "/Game/UI/W_SlapMeter.W_SlapMeter_C" false))
      (for _array_element _foundwidgets
        (`UserWidget.PauseAnimation` _array_element (`/Game/UI/W_SlapMeter.SlapMeter` _array_element))
        (`|SpawnActorFromClass` "/Game/Blueprints/BP_Force.BP_Force_C" (`KismetMathLibrary.MakeTransform` _returnvalue_location _returnvalue_rotation) "Undefined" "MultiplyWithRoot" null null)
        (`GameplayStatics.PlaySoundAtLocation` "/Game/Blueprints/Salp.Salp" _returnvalue_location (struct) 1.0 1.0 0.0 null null null null)))))

(fn `UserConstructionScript`)